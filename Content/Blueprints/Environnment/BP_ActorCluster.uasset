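; BP_ActorCluster is a level actor that resets a group of linked actors when the player respawns before reaching its linked checkpoint.
; On BeginPlay it records each linked actor's transform and binds to the game manager's respawn event.
; On respawn, it spawns fresh same-class copies at those transforms, destroys the old ones, and passes the new list to an optional kill-enemy activator.
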(event Custom|OnPlayerRespawn
  (if (not (Variables|/Game/Blueprints/Environnment/BP_Checkpoint.BP_Checkpoint_C|GetbIsChecked? (Variables|Default|GetLinkedCheckPoint)))
    (CallFunction|RespawnActors)))

(event EventBeginPlay
  (CallFunction|SetupEvents)
  (CallFunction|SetupTransforms))

(fn ConstructionScript)

(fn SetupEvents
  (EventDispatchers|BindEventtoOnPlayerRespawn (CallFunction|GetGameManager) (EventDispatchers|CreateEvent :!event Custom|OnPlayerRespawn)))

(fn SetupTransforms
  (for _array_element (Variables|Default|GetLinkedActor)
    (Utilities|Array|Add (Variables|Default|GetOriginalTransforms) (Transformation|GetActorTransform _array_element))))

(fn RespawnActors
  (Utilities|Array|Clear (Variables|Default|GetTempLinkedActors))
  (for (_array_element _array_index) (Variables|Default|GetLinkedActor)
    (bind _returnvalue (Game|SpawnActorfromClass (Utilities|GetClass _array_element) (Utilities|Array|Get(acopy) (Variables|Default|GetOriginalTransforms) _array_index) "AdjustIfPossibleButAlwaysSpawn" 0 0))
    (Utilities|Array|Add (Variables|Default|GetTempLinkedActors) _returnvalue)
    (Actor|DestroyActor _array_element))
  (Variables|Default|SetLinkedActor (Variables|Default|GetTempLinkedActors))
  (if (Utilities|IsValid (Variables|Default|GetLinkedKillEnemyActivator))
    (Variables|/Game/Blueprints/Environnment/Activators/BP_ActivatorKillerEnemy.BP_ActivatorKillerEnemy_C|SetTempLinkedEnemies (Variables|Default|GetLinkedKillEnemyActivator) (Variables|Default|GetTempLinkedActors))))