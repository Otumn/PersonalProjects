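; BP_MissionObjective is a placed mission marker that shows its action text while its assigned index is the current objective.
; It listens to the Game Manager's objective-set event, toggling marker visibility and collapsing the trigger box to zero scale when inactive.
; Player overlap, or interaction through the interactible component, sets the next objective.
; On Tick, the active marker faces the camera and scales with camera distance.
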(event OnComponentBeginOverlap(Box)
  (params (OverlappedComponent :type Primitive%20Component%20Object%20Reference) (OtherActor :type Actor%20Object%20Reference) (OtherComp :type Primitive%20Component%20Object%20Reference) (OtherBodyIndex :type Integer) (bFromSweep :type Boolean) (SweepResult :type Hit%20Result%20Structure%20%28by%20ref%29))
  (if (and (== OtherActor (Game|Player|GetPlayerPawn 0)) (not (Variables|Default|GetbHasToInteract?)))
    (Default|CallOnObjectiveSet (CallFunction|GetGameManager) (Variables|Default|GetNextMissionObjective))))

(event OnInteracted(BP_InteractibleComponent)
  (Default|CallOnObjectiveSet (CallFunction|GetGameManager) (Variables|Default|GetNextMissionObjective)))

(event Custom|OnNewObjective
  (params (Index :type Integer))
  (bind _output_get (Variables|Default|SetbObjectiveActive? (== Index (Variables|Default|GetAssignedMissionIndex))))
  (Rendering|SetVisibility (Variables|Default|GetObjHolder) _output_get true)
  (Transformation|SetWorldScale3D (Variables|Default|GetBox) (Math|Vector|SelectVector (Variables|Default|GetBoxOriginalScale) "0, 0, 0" _output_get)))

(event EventBeginPlay
  (bind _bp_interactiblecomponent (Variables|Default|GetBP_InteractibleComponent))
  (EventDispatchers|BindEventtoOnObjectiveSet (CallFunction|GetGameManager) (EventDispatchers|CreateEvent :!event Custom|OnNewObjective))
  (Variables|Default|SetBoxOriginalScale (Transformation|GetWorldScale (Variables|Default|GetBox)))
  (if (not (Variables|Default|GetbHasToInteract?))
    (Variables|/Game/Blueprints/Components/BP_InteractibleComponent.BP_InteractibleComponent_C|SetActionName _bp_interactiblecomponent "")
    (Variables|/Game/Blueprints/Components/BP_InteractibleComponent.BP_InteractibleComponent_C|SetItemName _bp_interactiblecomponent "")))

(event EventTick
  (params (DeltaSeconds :type Float%20%28single-precision%29))
  (CallFunction|TextManager))

(fn ConstructionScript
  (Rendering|Components|TextRender|SetText (Variables|Default|GetTextRender) (Utilities|Text|ToText(String) (Variables|Default|GetObjectiveAction))))

(fn TextManager
  (bind _returnvalue (Game|GetPlayerCameraManager 0))
  (bind _objholder (Variables|Default|GetObjHolder))
  (bind _maxtextsize (Variables|Default|GetMaxTextSize))
  (bind _mintextsize (Variables|Default|GetMinTextSize))
  (bind _minplayerdist (Variables|Default|GetMinPlayerDist))
  (bind _maxplayerdist (Variables|Default|GetMaxPlayerDist))
  (bind _objholder_2 (Variables|Default|GetObjHolder))
  (bind _returnvalue_2 (Transformation|GetWorldLocation _objholder_2))
  (bind _transformcomponent (Variables|/Script/Engine.PlayerCameraManager|GetTransformComponent _returnvalue))
  (bind _returnvalue_3 (Transformation|GetWorldLocation _transformcomponent))
  (bind _returnvalue_4 (Math|Vector|Distance(Vector) _returnvalue_2 _returnvalue_3))
  (bind _returnvalue_5 (Math|Float|NormalizetoRange _returnvalue_4 _minplayerdist _maxplayerdist))
  (bind _returnvalue_6 (Math|Float|Lerp _mintextsize _maxtextsize _returnvalue_5))
  (if (Variables|Default|GetbObjectiveActive?)
    (Transformation|SetWorldScale3D (Variables|Default|GetObjHolder) (Math|Vector|MakeVector _returnvalue_6 _returnvalue_6 _returnvalue_6))
    (Transformation|SetWorldRotation _objholder (Math|Rotator|FindLookatRotation (Transformation|GetWorldLocation _objholder) (Transformation|GetActorLocation (Game|GetPlayerCameraManager 0))) false false)))