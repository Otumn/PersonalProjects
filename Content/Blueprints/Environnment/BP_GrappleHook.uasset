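; BP_GrappleHook is an environment grapple hook point that shows visual markers and rotates to face the player pawn every tick.
; WakeUp and Sleep show and hide the base widget, and both leave actor tick enabled.
; SetInRange and UnsetInRange toggle the in-range widget and the IsInRange flag; the actor does no range detection itself, so these events depend on outside callers.
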(event Custom|WakeUp
  (Actor|Tick|SetActorTickEnabled true)
  (Rendering|SetVisibility (Variables|Default|GetBaseWidget) true false))

(event Custom|Sleep
  (Actor|Tick|SetActorTickEnabled true)
  (Rendering|SetVisibility (Variables|Default|GetBaseWidget) false false))

(event Custom|SetInRange
  (Rendering|SetVisibility (Variables|Default|GetInRangeWidget) true false)
  (Variables|Default|SetisInRange? true))

(event Custom|UnsetInRange
  (Rendering|SetVisibility (Variables|Default|GetInRangeWidget) false false)
  (Variables|Default|SetisInRange? false))

(event EventTick
  (params (DeltaSeconds :type Float%20%28single-precision%29))
  (CallFunction|ActorFaceActor self (Game|Player|GetPlayerPawn 0)))

(fn ConstructionScript)