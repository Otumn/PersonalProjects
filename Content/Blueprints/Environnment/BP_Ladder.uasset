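; BP_Ladder is an interactable ladder that teleports the player between its two ends instead of animating a climb.
; When its BP_InteractibleComponent fires OnInteracted, it compares the height of player pawn 0 to the TopSpawn component.
; A pawn below TopSpawn teleports to TopSpawn's location and rotation, and otherwise to those of BotSpawn.
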(event OnInteracted(BP_InteractibleComponent)
  (bind _topspawn (Variables|Default|GetTopSpawn))
  (bind _botspawn (Variables|Default|GetBotSpawn))
  (if (< (.Z (Math|Vector|BreakVector (Transformation|GetActorLocation (Game|Player|GetPlayerPawn 0)))) (.Z (Math|Vector|BreakVector (Transformation|GetWorldLocation (Variables|Default|GetTopSpawn)))))
    (Transformation|SetActorLocationAndRotation (Game|Player|GetPlayerPawn 0) (Transformation|GetWorldLocation _topspawn) (Transformation|GetWorldRotation _topspawn) false true)
    (else
      (Transformation|SetActorLocationAndRotation (Game|Player|GetPlayerPawn 0) (Transformation|GetWorldLocation _botspawn) (Transformation|GetWorldRotation _botspawn) false true))))

(fn ConstructionScript)