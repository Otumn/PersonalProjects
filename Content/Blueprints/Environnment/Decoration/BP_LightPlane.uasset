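; BP_LightPlane is a decorative light fixture that pairs a rect light with a visible plane mesh.
; The construction script sets the light's color, intensity, barn doors, source size and attenuation radius from exposed variables.
; The same size, color and scaled-down intensity drive the plane's scale and material parameters, so the glowing surface matches the light it casts.
; It has no runtime logic.
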(event EventBeginPlay)

(event Collision|EventActorBeginOverlap
  (params (OtherActor :type Actor%20Object%20Reference)))

(event EventTick
  (params (DeltaSeconds :type Float%20%28single-precision%29)))

(fn ConstructionScript
  (bind _rectlight (Variables|Default|GetRectLight))
  (bind _plane (Variables|Default|GetPlane))
  (Utilities|FlowControl|Sequence
    (:then_0
      (Rendering|Components|Light|SetLightColor _rectlight (Variables|Default|GetColor) true)
      (Rendering|Components|Light|SetIntensity _rectlight (Variables|Default|GetIntensity))
      (Class|RectLightComponent|SetBarnDoorAngle _rectlight (Variables|Default|GetAngle))
      (Class|RectLightComponent|SetBarnDoorLength _rectlight (Variables|Default|GetLenght))
      (Class|RectLightComponent|SetSourceWidth _rectlight (* (Variables|Default|GetY) 1e+02))
      (Class|RectLightComponent|SetSourceHeight _rectlight (* (Variables|Default|GetZ) 1e+02))
      (Rendering|Lighting|SetAttenuationRadius _rectlight (Variables|Default|GetRadius)))
    (:then_1
      (Rendering|Material|SetVectorParameterValueonMaterials _plane "Color" (Math|Conversions|ToVector(LinearColor) (Variables|Default|GetColor)))
      (Transformation|SetRelativeScale3D _plane (Math|Vector|MakeVector (Variables|Default|GetZ) (Variables|Default|GetY) 0.0))
      (Rendering|Material|SetScalarParameterValueonMaterials _plane "Intensity" (* (Variables|Default|GetIntensity) 0.0002)))))