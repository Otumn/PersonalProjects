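; Decoration Blueprint that fills a rectangular wall area with randomly scattered static meshes.
; The construction script only resizes a thin Box to the X/Y dimensions of that area.
; CreateMeshes clears previous pieces, then adds components with random mesh, material, depth, in-plane position, stepped roll and Y/Z scale.
; LinkedMeshes tracks the spawned components so DeleteMeshes can destroy them.
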(fn ConstructionScript
  (Transformation|SetRelativeScale3D (Variables|Default|GetBox) (Math|Vector|MakeVector 0.01 (Variables|Default|GetX) (Variables|Default|GetY))))

(fn CreateMeshes
  (bind _xplacemenentrange (Variables|Placement|GetXPlacemenentRange))
  (bind _scalerange (Variables|Placement|GetScaleRange))
  (bind _possiblemeshes (Variables|Default|GetPossibleMeshes))
  (bind _possiblesmaterials (Variables|Default|GetPossiblesMaterials))
  (bind _x (Variables|Default|GetX))
  (bind _y (Variables|Default|GetY))
  (bind _scalerange_2 (Variables|Placement|GetScaleRange))
  (CallFunction|DeleteMeshes)
  (for _index (range 0 (Variables|Default|GetNumberOfMeshes))
    (bind _returnvalue (AddComponent|AddStaticMeshComponent false (Math|Transform|MakeTransform (Math|Vector|MakeVector (Math|Random|RandomFloatinRange (* _xplacemenentrange -1.0) _xplacemenentrange) (Math|Random|RandomFloatinRange (* _x -5e+01) (* _x 5e+01)) (Math|Random|RandomFloatinRange (* _y -5e+01) (* _y 5e+01))) (Math|Rotator|MakeRotator (Utilities|Select :Index (Math|Random|RandomIntegerinRange 0 2) :Option%200 0.0 :Option%201 9e+01 :Option%202 1.8e+02 :Option%203 3.6e+02) 0.0 0.0) (Math|Vector|MakeVector 1.0 (Math|Random|RandomFloatinRange (- 1.0 _scalerange_2) (+ _scalerange_2 1.0)) (Math|Random|RandomFloatinRange (- 1.0 _scalerange) (+ _scalerange 1.0))))))
    (Components|StaticMesh|SetStaticMesh _returnvalue (Utilities|Array|Get(acopy) _possiblemeshes (Math|Random|RandomIntegerinRange 0 (Utilities|Array|Length _possiblemeshes))))
    (Rendering|Material|SetMaterial _returnvalue 0 (Utilities|Array|Get(acopy) _possiblesmaterials (Math|Random|RandomIntegerinRange 0 (Utilities|Array|Length _possiblesmaterials))))
    (Utilities|Array|Add (Variables|Default|GetLinkedMeshes) _returnvalue)))

(fn DeleteMeshes
  (bind _arrayelement (Utilities|Array|ReverseforEachLoop (Variables|Default|GetLinkedMeshes))
    (:LoopBody
      (Components|DestroyComponent _arrayelement))
    (:Completed
      (Utilities|Array|Clear (Variables|Default|GetLinkedMeshes)))))