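; Checkpoint actor that registers itself with the game manager when the player pawn overlaps its box.
; A checkpoint flagged as the first one also registers itself shortly after BeginPlay, following a brief delay.
; RegisterCheckPoint uses a checked flag so each checkpoint notifies the manager only once, passing itself through CallOnCheckPointReached.
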(event OnComponentBeginOverlap(Box)
  (params (OverlappedComponent :type Primitive%20Component%20Object%20Reference) (OtherActor :type Actor%20Object%20Reference) (OtherComp :type Primitive%20Component%20Object%20Reference) (OtherBodyIndex :type Integer) (bFromSweep :type Boolean) (SweepResult :type Hit%20Result%20Structure%20%28by%20ref%29))
  (if (== OtherActor (Game|Player|GetPlayerPawn 0))
    (CallFunction|RegisterCheckPoint)))

(event EventBeginPlay
  (Utilities|FlowControl|Delay 0.2)
  (if (Variables|Default|GetbIsFirstCheckPoint?)
    (CallFunction|RegisterCheckPoint)))

(fn ConstructionScript)

(fn RegisterCheckPoint
  (if (not (Variables|Default|GetbIsChecked?))
    (Variables|Default|SetbIsChecked? true)
    (Default|CallOnCheckPointReached (CallFunction|GetGameManager) self)))