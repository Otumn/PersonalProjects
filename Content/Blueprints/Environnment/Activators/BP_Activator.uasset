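; BP_Activator is an environment activator that switches a list of linked actors on and off.
; ActivateActors and DesactivateActors loop over Activables, find each actor's BP_ActivableComponent and call its activate or deactivate function.
; On BeginPlay it binds to the game manager's player respawn event, so a respawn deactivates the actors unless the linked checkpoint has been checked.
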(event Custom|ActivateActors
  (for _array_element (Variables|Default|GetActivables)
    (if (.HasComponent (CallFunction|DoesActorHasComponent? _array_element "/Game/Blueprints/Components/BP_ActivableComponent.BP_ActivableComponent_C"))
      (bind _asbp_activable_component (Utilities|Casting|CastToBP_ActivableComponent (.ReturnedComponent (CallFunction|DoesActorHasComponent? _array_element "/Game/Blueprints/Components/BP_ActivableComponent.BP_ActivableComponent_C"))))
      (Default|CallActivateLinkedObject _asbp_activable_component))))

(event Custom|OnPlayerRespawns
  (if (not (Variables|/Game/Blueprints/Environnment/BP_Checkpoint.BP_Checkpoint_C|GetbIsChecked? (Variables|Default|GetLinkedCheckPoint)))
    (CallFunction|DesactivateActors)))

(event Custom|DesactivateActors
  (for _array_element (Variables|Default|GetActivables)
    (if (.HasComponent (CallFunction|DoesActorHasComponent? _array_element "/Game/Blueprints/Components/BP_ActivableComponent.BP_ActivableComponent_C"))
      (bind _asbp_activable_component (Utilities|Casting|CastToBP_ActivableComponent (.ReturnedComponent (CallFunction|DoesActorHasComponent? _array_element "/Game/Blueprints/Components/BP_ActivableComponent.BP_ActivableComponent_C"))))
      (Default|CallDeactivateLinkedObject _asbp_activable_component))))

(event EventBeginPlay
  (CallFunction|SetupEvents))

(fn ConstructionScript)

(fn SetupEvents
  (EventDispatchers|BindEventtoOnPlayerRespawn (CallFunction|GetGameManager) (EventDispatchers|CreateEvent :!event Custom|OnPlayerRespawns)))