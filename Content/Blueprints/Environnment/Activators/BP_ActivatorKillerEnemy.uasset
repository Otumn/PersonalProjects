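; BP_ActivatorKillerEnemy is an activator that triggers its actors once every linked enemy has been killed.
; On BeginPlay it subscribes to the game manager's actor-killed event and copies LinkedEnemies into a working list.
; Each killed actor found in that list is removed, and ActivateActors runs when the list becomes empty.
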(event Custom|OnActorKilled
  (params (Actor :type Actor%20Object%20Reference))
  (if (Utilities|Array|ContainsItem (Variables|Default|GetTempLinkedEnemies) Actor)
    (Utilities|Array|RemoveItem (Variables|Default|GetTempLinkedEnemies) Actor)
    (if (== (Utilities|Array|Length (Variables|Default|GetTempLinkedEnemies)) 0)
      (CallFunction|ActivateActors))))

(event EventBeginPlay
  (|CallParentFunction)
  (CallFunction|SetupEvents0)
  (Variables|Default|SetTempLinkedEnemies (Variables|Default|GetLinkedEnemies)))

(fn ConstructionScript
  (|CallParentFunction))

(fn SetupEvents0
  (EventDispatchers|BindEventtoOnActorKilled (CallFunction|GetGameManager) (EventDispatchers|CreateEvent :!event Custom|OnActorKilled)))