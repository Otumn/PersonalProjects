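; BP_GiantFan is an environmental hazard: a giant fan whose spinning propeller kills the player on contact.
; Tick rotates the Propeller around its roll axis at a configurable Speed, scaled by delta time.
; The construction script applies StartRotation as the propeller's initial roll.
; When the propeller begins overlapping the player pawn, it casts it to BP_SprinterPlayer and calls RequestKillPlayer.
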(event OnComponentHit(Propeller)
  (params (HitComponent :type Primitive%20Component%20Object%20Reference) (OtherActor :type Actor%20Object%20Reference) (OtherComp :type Primitive%20Component%20Object%20Reference) (NormalImpulse :type Vector :default "0, 0, 0") (Hit :type Hit%20Result%20Structure%20%28by%20ref%29)))

(event OnComponentBeginOverlap(Propeller)
  (params (OverlappedComponent :type Primitive%20Component%20Object%20Reference) (OtherActor :type Actor%20Object%20Reference) (OtherComp :type Primitive%20Component%20Object%20Reference) (OtherBodyIndex :type Integer) (bFromSweep :type Boolean) (SweepResult :type Hit%20Result%20Structure%20%28by%20ref%29))
  (if (== (Game|Player|GetPlayerPawn 0) OtherActor)
    (Default|RequestKillPlayer (.AsBP%20Sprinter%20Player (Utilities|Casting|CastToBP_SprinterPlayer OtherActor)))))

(event EventTick
  (params (DeltaSeconds :type Float%20%28single-precision%29))
  (Transformation|AddRelativeRotation (Variables|Default|GetPropeller) (Math|Rotator|MakeRotator (* DeltaSeconds (Variables|Default|GetSpeed) 1.0) 0.0 0.0) false false))

(fn ConstructionScript
  (Transformation|SetRelativeRotation (Variables|Default|GetPropeller) (Math|Rotator|MakeRotator (Variables|Default|GetStartRotation) 0.0 0.0) false false))