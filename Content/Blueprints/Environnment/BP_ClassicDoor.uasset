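; Interactable hinged door that swings open and closed, or only budges when flagged as WontBudge.
; Each interaction alternates playing and reversing a timeline that yaws the door root; stuck doors replay a separate budge timeline instead.
; A dot product between door and camera forward vectors picks the swing direction before opening or budging.
; The construction script sets the cube's material, size and hinge offset, plus the interaction component's item and action names.
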(event OnInteracted(BP_InteractibleComponent)
  (bind _targetopenrotation (Variables|Default|GetTargetOpenRotation))
  (bind _targetbudgerotation (Variables|Default|GetTargetBudgeRotation))
  (if (Variables|Default|GetbWontBudge?)
    (CallFunction|SetInvertOpening)
    (bind _alpha (Timeline|BudgeTimeline PlayFromStart)
      (:Update
        (Transformation|SetRelativeRotation (Variables|Default|GetDoorRoot) (Math|Rotator|MakeRotator 0.0 0.0 (Math|Float|Lerp 0.0 (Math|Float|SelectFloat _targetbudgerotation (* _targetbudgerotation -1.0) (Variables|Default|GetbInvertOpening?)) _alpha)) false false)))
    (else
      (Utilities|FlowControl|FlipFlop
        (:A
          (CallFunction|SetInvertOpening)
          (bind _alpha_2 (Timeline|OpenTimeline Play)
            (:Update
              (Transformation|SetRelativeRotation (Variables|Default|GetDoorRoot) (Math|Rotator|MakeRotator 0.0 0.0 (Math|Float|Lerp 0.0 (Math|Float|SelectFloat _targetopenrotation (* _targetopenrotation -1.0) (Variables|Default|GetbInvertOpening?)) _alpha_2)) false false))))
        (:B
          (Timeline|OpenTimeline Reverse))))))

(event EventBeginPlay
  (CallFunction|SetupTimelinesRate))

(fn ConstructionScript
  (bind _x (Variables|Default|GetX))
  (bind _y (Variables|Default|GetY))
  (bind _bp_interactiblecomponent (Variables|Default|GetBP_InteractibleComponent))
  (bind _returnvalue (* _y 2.5))
  (bind _returnvalue_2 (* _x 1.6))
  (Utilities|FlowControl|Sequence
    (:then_0
      (Rendering|Material|SetMaterial (Variables|Default|GetCube) 0 (Variables|Default|GetMaterial)))
    (:then_1
      (Transformation|SetRelativeScale3D (Variables|Default|GetCube) (Math|Vector|MakeVector 0.1 _returnvalue_2 _returnvalue))
      (Transformation|SetRelativeLocation (Variables|Default|GetCube) (Math|Vector|MakeVector 0.0 (* _returnvalue_2 5e+01) (* _returnvalue 5e+01)) false false))
    (:then_2
      (Variables|/Game/Blueprints/Components/BP_InteractibleComponent.BP_InteractibleComponent_C|SetItemName _bp_interactiblecomponent (Variables|Default|GetName))
      (Variables|/Game/Blueprints/Components/BP_InteractibleComponent.BP_InteractibleComponent_C|SetActionName _bp_interactiblecomponent (Variables|Default|GetAction)))))

(fn SetupTimelinesRate
  (Components|Timeline|SetPlayRate (Variables|Default|GetOpenTimeline) (Variables|Default|GetOpenRate))
  (Components|Timeline|SetPlayRate (Variables|Default|GetBudgeTimeline) (Variables|Default|GetBudgerate)))

(fn SetInvertOpening
  (Variables|Default|SetbInvertOpening? (< (Math|Vector|DotProduct (Math|Vector|GetForwardVector (Variables|Default|GetCube)) (Transformation|GetActorForwardVector (Game|GetPlayerCameraManager 0))) 0.0)))