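; Elevator actor that moves its Cylinder component to a Target location when the player pawn overlaps the ActivationBox.
; A timeline lerps the world location from the captured start position, with play rate set from TimeToGetToTarget.
; It binds to the game manager's player respawn event and, if already activated, resets the timeline time and replays the ride.
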(event OnComponentBeginOverlap(ActivationBox)
  (params (OverlappedComponent :type Primitive%20Component%20Object%20Reference) (OtherActor :type Actor%20Object%20Reference) (OtherComp :type Primitive%20Component%20Object%20Reference) (OtherBodyIndex :type Integer) (bFromSweep :type Boolean) (SweepResult :type Hit%20Result%20Structure%20%28by%20ref%29))
  (if (== (Game|Player|GetPlayerPawn 0) OtherActor)
    (CallFunction|StartElevator)
    (Variables|Default|SetbHasBeenActivated? true)))

(event Custom|StartElevator
  (Components|Timeline|SetPlayRate (Variables|Default|GetMovementTimeline) (/ 1.0 (Variables|Default|GetTimeToGetToTarget)))
  (Variables|Default|SetStartLocation (Transformation|GetWorldLocation (Variables|Default|GetCylinder)))
  (bind _alpha (Timeline|MovementTimeline PlayFromStart)
    (:Update
      (Transformation|SetWorldLocation (Variables|Default|GetCylinder) (Math|Vector|Lerp(Vector) (Variables|Default|GetStartLocation) (Transformation|GetWorldLocation (Variables|Default|GetTarget)) _alpha) false false))))

(event Custom|OnPlayerRespawn
  (if (Variables|Default|GetbHasBeenActivated?)
    (Utilities|FlowControl|Sequence
      (:then_0
        (bind _alpha (Timeline|MovementTimeline SetNewTime)
          (:Update
            (Transformation|SetWorldLocation (Variables|Default|GetCylinder) (Math|Vector|Lerp(Vector) (Variables|Default|GetStartLocation) (Transformation|GetWorldLocation (Variables|Default|GetTarget)) _alpha) false false))))
      (:then_1
        (Timeline|MovementTimeline Play)))))

(event EventBeginPlay
  (CallFunction|SetupEvents))

(fn ConstructionScript)

(fn SetupEvents
  (EventDispatchers|BindEventtoOnPlayerRespawn (CallFunction|GetGameManager) (EventDispatchers|CreateEvent :!event Custom|OnPlayerRespawn)))