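; BP_NumberWheel is an interactable ten-digit number wheel in the Prison environment that advances one number each time it is used.
; Interaction starts a timeline that lerps the Rotator component's pitch in 36-degree steps along the shortest path, so 9 wraps smoothly to 0.
; An IsTurning flag ignores input mid-turn, and CurrentNumber updates only when the timeline finishes, with TurnRate setting the play rate.
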(event OnInteracted(BP_InteractibleComponent)
  (if (not (Variables|Default|GetbIsTurning?))
    (Variables|Default|SetbIsTurning? true)
    (Variables|Default|SetTargetRot (* (CallFunction|GetNextNumber) 36.0))
    (Variables|Default|SetStartRot (* (Variables|Default|GetCurrentNumber) 36.0))
    (bind _alpha (Timeline|TurnWheelTimeline PlayFromStart)
      (:Update
        (Transformation|SetRelativeRotation (Variables|Default|GetRotator) (Math|Rotator|Lerp(Rotator) (Math|Rotator|MakeRotator 0.0 (Variables|Default|GetStartRot) 0.0) (Math|Rotator|MakeRotator 0.0 (Variables|Default|GetTargetRot) 0.0) _alpha true) true false))
      (:Finished
        (Variables|Default|SetCurrentNumber (CallFunction|GetNextNumber))
        (Variables|Default|SetbIsTurning? false)))))

(event EventBeginPlay
  (Components|Timeline|SetPlayRate (Variables|Default|GetTurnWheelTimeline) (Variables|Default|GetTurnRate)))

(fn ConstructionScript)

(fn GetNextNumber
  (bind _currentnumber (Variables|Default|GetCurrentNumber))
  (bind _returnvalue (+ _currentnumber 1))
  (if (> _returnvalue 9)
    (return 0)
    (else
      (return _returnvalue))))