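; BP_PrisonLock is a four-wheel combination lock for the prison level that checks the entered code when the player interacts with it.
; Interaction runs a timeline showing a checking message, then CheckNumbers compares each wheel's current number to its expected digit and the text display shows success or failure.
; It sets objective 0 shortly after BeginPlay and objective 1 on a correct code, and a CanCheck flag blocks repeat checks until reset.
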(event OnInteracted(BP_InteractibleComponent)
  (if (Variables|Default|GetbCanCheck?)
    (Variables|Default|SetbCanCheck? false)
    (Timeline|CheckTimeline PlayFromStart
      (:Update
        (Rendering|Components|TextRender|SetText (Variables|Default|GetTextRender) (Utilities|Text|MakeLiteralText "Checking...")))
      (:Finished
        (if (CallFunction|CheckNumbers)
          (Rendering|Components|TextRender|SetText (Variables|Default|GetTextRender) (Utilities|Text|MakeLiteralText "Opening door"))
          (Default|CallOnObjectiveSet (CallFunction|GetGameManager) 1)
          (else
            (Rendering|Components|TextRender|SetText (Variables|Default|GetTextRender) (Utilities|Text|MakeLiteralText "Invalid code"))))
        (Utilities|FlowControl|Delay 2.0)
        (Variables|Default|SetbCanCheck? true)
        (Rendering|Components|TextRender|SetText (Variables|Default|GetTextRender) (Utilities|Text|MakeLiteralText "Waiting..."))))))

(event EventBeginPlay
  (Utilities|FlowControl|Delay 0.2)
  (Default|CallOnObjectiveSet (CallFunction|GetGameManager)))

(fn ConstructionScript)

(fn CheckNumbers
  (return (Math|Boolean|ANDBoolean (== (Variables|/Game/Blueprints/Environnment/Prison/BP_NumberWheel.BP_NumberWheel_C|GetCurrentNumber (Variables|Default|GetWheel1)) (Variables|Default|GetNumber1)) (== (Variables|/Game/Blueprints/Environnment/Prison/BP_NumberWheel.BP_NumberWheel_C|GetCurrentNumber (Variables|Default|GetWheel2)) (Variables|Default|GetNumber2)) (== (Variables|/Game/Blueprints/Environnment/Prison/BP_NumberWheel.BP_NumberWheel_C|GetCurrentNumber (Variables|Default|GetWheel3)) (Variables|Default|GetNumber3)) (== (Variables|/Game/Blueprints/Environnment/Prison/BP_NumberWheel.BP_NumberWheel_C|GetCurrentNumber (Variables|Default|GetWheel4)) (Variables|Default|GetNumber4)))))