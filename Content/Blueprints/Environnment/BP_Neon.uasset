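; BP_Neon is an environment neon panel whose texture, colors and glow are configurable through its variables.
; Its Construction Script creates a dynamic instance of M_Pannel on the first material slot of the Plane component.
; It then passes the texture, plus separate color and emissive values for the inside text and the outline, into the material parameters.
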(fn ConstructionScript
  (bind _returnvalue (Rendering|Material|CreateDynamicMaterialInstance (Variables|Default|GetPlane) 0 "/Game/Materials/M_Pannel.M_Pannel" "None" :!class /Script/Engine.PrimitiveComponent))
  (Rendering|Material|SetTextureParameterValue _returnvalue "Texture" (Variables|Default|GetTexture))
  (Rendering|Material|SetVectorParameterValue _returnvalue "InsideColor" (Variables|Default|GetTextColor) :!class /Script/Engine.MaterialInstanceDynamic)
  (Rendering|Material|SetVectorParameterValue _returnvalue "OutlineColor" (Variables|Default|GetOutlineColor) :!class /Script/Engine.MaterialInstanceDynamic)
  (Rendering|Material|SetScalarParameterValue _returnvalue "InsideEmissive" (Variables|Default|GetTextEmissive) :!class /Script/Engine.MaterialInstanceDynamic)
  (Rendering|Material|SetScalarParameterValue _returnvalue "OutlineEmissive" (Variables|Default|GetOutlineEmissive) :!class /Script/Engine.MaterialInstanceDynamic))