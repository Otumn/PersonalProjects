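; BP_ElectricWall is a resizable electric wall hazard that kills the player on contact.
; The construction script uses X and Y to scale the electric plane, back panel and kill box, and to place and stretch the left and right side pieces.
; It also multiplies the material's tile parameters by the size, so tiling scales with the wall.
; When the player pawn overlaps KillBox, it calls RequestKillPlayer on BP_SprinterPlayer.
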(event OnComponentBeginOverlap(KillBox)
  (params (OverlappedComponent :type Primitive%20Component%20Object%20Reference) (OtherActor :type Actor%20Object%20Reference) (OtherComp :type Primitive%20Component%20Object%20Reference) (OtherBodyIndex :type Integer) (bFromSweep :type Boolean) (SweepResult :type Hit%20Result%20Structure%20%28by%20ref%29))
  (if (== (Game|Player|GetPlayerPawn 0) OtherActor)
    (Default|RequestKillPlayer (.AsBP%20Sprinter%20Player (Utilities|Casting|CastToBP_SprinterPlayer OtherActor)))))

(fn ConstructionScript
  (Utilities|FlowControl|Sequence
    (:then_0
      (Transformation|SetRelativeScale3D (Variables|Default|GetElectricPlane) (Math|Vector|MakeVector (Variables|Default|GetX) (Variables|Default|GetY) 1.0)))
    (:then_1
      (Rendering|Material|SetScalarParameterValueonMaterials (Variables|Default|GetElectricPlane) "XTiles" (* (Variables|Default|GetX) (Variables|Default|GetXTiles)))
      (Rendering|Material|SetScalarParameterValueonMaterials (Variables|Default|GetElectricPlane) "YTiles" (* (Variables|Default|GetY) (Variables|Default|GetYTiles))))
    (:then_2
      (Transformation|SetRelativeLocation (Variables|Default|GetLeft) (Math|Vector|MakeVector (+ (* (Variables|Default|GetX) -5e+01) -5.0) 0.0 0.0) false false)
      (Transformation|SetRelativeScale3D (Variables|Default|GetLeft) (Math|Vector|MakeVector 0.1 (Variables|Default|GetY) 0.15625)))
    (:then_3
      (Transformation|SetRelativeLocation (Variables|Default|GetRight) (Math|Vector|MakeVector (+ (* (Variables|Default|GetX) 5e+01) 5.0) 0.0 0.0) false false)
      (Transformation|SetRelativeScale3D (Variables|Default|GetRight) (Math|Vector|MakeVector 0.1 (Variables|Default|GetY) 0.15625)))
    (:then_4
      (Transformation|SetRelativeScale3D (Variables|Default|GetBack) (Math|Vector|MakeVector (Variables|Default|GetX) (Variables|Default|GetY) 0.0625)))
    (:then_5
      (Transformation|SetRelativeScale3D (Variables|Default|GetKillBox) (Math|Vector|MakeVector (* (Variables|Default|GetX) 1.7) (* (Variables|Default|GetY) 1.6) 0.75)))))