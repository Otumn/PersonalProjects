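; BP_PlayerDeathLogic is a logic Blueprint that shows and hides the death screen when the player dies and respawns.
; On BeginPlay it binds handlers to the game manager's player death and respawn events.
; On death it creates a BPW_DeathUI widget for the first player, adds it to the viewport and plays its appear animation.
; On respawn it removes the widget and clears the reference.
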(event Custom|OnPlayerDeath
  (bind _returnvalue (UserInterface|CreateWidget "/Game/Blueprints/WIdget/BPW_DeathUI.BPW_DeathUI_C" (Game|GetPlayerController 0)))
  (bind _output_get (Variables|Default|SetDeathUI _returnvalue))
  (UserInterface|Viewport|AddtoViewport _output_get 0)
  (UserInterface|Animation|PlayAnimation _output_get (Variables|/Game/Blueprints/WIdget/BPW_DeathUI.BPW_DeathUI_C|GetAppearAnimation _output_get) 0.0 1 "Forward" 1.0))

(event Custom|OnPlayerRespawn
  (Widget|RemovefromParent (Variables|Default|GetDeathUI))
  (Variables|Default|SetDeathUI 0))

(event EventBeginPlay
  (CallFunction|SetupEvents))

(fn ConstructionScript)

(fn SetupEvents
  (EventDispatchers|BindEventtoOnPlayerDeath (CallFunction|GetGameManager) (EventDispatchers|CreateEvent :!event Custom|OnPlayerDeath))
  (EventDispatchers|BindEventtoOnPlayerRespawn (CallFunction|GetGameManager) (EventDispatchers|CreateEvent :!event Custom|OnPlayerRespawn)))