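; Checkpoint logic actor that records the player's latest checkpoint and respawns them there.
; On begin play it binds to the game manager's checkpoint-reached and player-respawn events.
; A newly reached checkpoint becomes current only if it is not already in the passed list, so revisiting older ones never moves progress back.
; On respawn it teleports the player pawn to that checkpoint's respawn point and aligns control rotation with it.
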(event Custom|OnCheckPointReached
  (params (CheckPoint :type BP%20Checkpoint%20Object%20Reference))
  (if (not (Utilities|Array|ContainsItem (Variables|Default|GetPassedCheckPoints) CheckPoint))
    (Variables|Default|SetCurrentCheckPoint CheckPoint)
    (Utilities|Array|Add (Variables|Default|GetPassedCheckPoints) CheckPoint)))

(event Custom|OnPlayerRespawn
  (bind _currentcheckpoint (Variables|Default|GetCurrentCheckPoint))
  (bind _respawnpoint (Variables|/Game/Blueprints/Environnment/BP_Checkpoint.BP_Checkpoint_C|GetRespawnPoint _currentcheckpoint))
  (bind _returnvalue (Transformation|GetWorldRotation _respawnpoint))
  (Transformation|Teleport (Game|Player|GetPlayerPawn 0) (Transformation|GetWorldLocation _respawnpoint) _returnvalue)
  (Pawn|SetControlRotation (Game|GetPlayerController 0) _returnvalue))

(event EventBeginPlay
  (CallFunction|SetupEvent))

(fn ConstructionScript)

(fn SetupEvent
  (EventDispatchers|BindEventtoOnCheckPointReached (CallFunction|GetGameManager) (EventDispatchers|CreateEvent :!event Custom|OnCheckPointReached))
  (EventDispatchers|BindEventtoOnPlayerRespawn (CallFunction|GetGameManager) (EventDispatchers|CreateEvent :!event Custom|OnPlayerRespawn)))