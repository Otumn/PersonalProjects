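; Behavior Tree task that makes a turret enemy turn to face the player while it waits out a reload.
; On execute it starts the BP_TurretEnemy reload effect, then succeeds after WaitTime.
; Each tick it interpolates the pawn's rotation toward player 0 on yaw only, at RotationSpeed, with pitch and roll targeting zero.
; An abort cancels the reload effect and finishes the abort.
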(event EventReceiveAbortAI
  (params (OwnerController :type AI%20Controller%20Object%20Reference) (ControlledPawn :type Pawn%20Object%20Reference))
  (Default|CancelReloadEffect (.AsBP%20Turret%20Enemy (Utilities|Casting|CastToBP_TurretEnemy ControlledPawn)))
  (Class|BTTaskBlueprintBase|FinishAbort))

(event EventReceiveExecuteAI
  (params (OwnerController :type AI%20Controller%20Object%20Reference) (ControlledPawn :type Pawn%20Object%20Reference))
  (Default|ReloadEffect (.AsBP%20Turret%20Enemy (Utilities|Casting|CastToBP_TurretEnemy ControlledPawn)))
  (Utilities|FlowControl|Delay (Variables|Default|GetWaitTime))
  (AI|BehaviorTree|FinishExecute true))

(event EventReceiveTickAI
  (params (OwnerController :type AI%20Controller%20Object%20Reference) (ControlledPawn :type Pawn%20Object%20Reference) (DeltaSeconds :type Float%20%28single-precision%29))
  (Transformation|SetActorRotation ControlledPawn (Math|Interpolation|RInterpTo (Transformation|GetActorRotation ControlledPawn) (Math|Rotator|MakeRotator 0.0 0.0 (.Yaw (Math|Rotator|BreakRotator (Math|Rotator|FindLookatRotation (Transformation|GetActorLocation ControlledPawn) (Transformation|GetActorLocation (Game|Player|GetPlayerPawn 0)))))) DeltaSeconds (Variables|Default|GetRotationSpeed))))