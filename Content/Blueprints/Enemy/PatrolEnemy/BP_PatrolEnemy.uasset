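; BP_PatrolEnemy is an enemy character that walks between patrol points and is destroyed when interacted with.
; On begin play or landing it loops through the points using AI MoveTo, timeline-smoothed turns and randomized waits.
; With patrol-on-start disabled, landing sends it to the first point to match that facing.
; Construction applies body color, walk speed and type name, shown on a label that turns to the camera every tick.
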(event OnInteracted(BP_InteractibleComponent)
  (Actor|DestroyActor))

(event Custom|PatrolThroughAllPoints
  (bind _alpha (Timeline|TurnAroundTimeline PlayFromStart)
    (:Update
      (Transformation|SetActorRotation (Math|Rotator|Lerp(Rotator) (Transformation|GetActorRotation) (Transformation|GetActorRotation (.DestActor (Utilities|Struct|BreakPatrolDestination (Utilities|Array|Get(acopy) (Variables|Default|GetPatrolPoints) (Variables|Default|GetCurrentPatrolIndex))))) _alpha true)))
    (:Finished
      (Utilities|FlowControl|Delay (+ (.WaitTime (Utilities|Struct|BreakPatrolDestination (Utilities|Array|Get(acopy) (Variables|Default|GetPatrolPoints) (Variables|Default|GetCurrentPatrolIndex)))) (Math|Random|RandomFloatinRange -1.5 1.5)))
      (Variables|Default|SetCurrentPatrolIndex (+ (Variables|Default|GetCurrentPatrolIndex) 1))
      (if (> (Variables|Default|GetCurrentPatrolIndex) (- (Utilities|Array|Length (Variables|Default|GetPatrolPoints)) 1))
        (Variables|Default|SetCurrentPatrolIndex 0))
      (AI|AIMoveTo (AI|GetAIController self) "0, 0, 0" (.DestActor (Utilities|Struct|BreakPatrolDestination (Utilities|Array|Get(acopy) (Variables|Default|GetPatrolPoints) (Variables|Default|GetCurrentPatrolIndex)))) -1.0 "Default" "Default" true true
        (:OnMoveFinished
          (CallFunction|PatrolThroughAllPoints))))))

(event Custom|BeginPatrolTest
  (if (Math|Boolean|ANDBoolean (> (Utilities|Array|Length (Variables|Default|GetPatrolPoints)) 0) (AI|Components|NavMovement|IsMovingonGround (Variables|Character|GetCharacterMovement)) (Variables|Default|GetPatrolingOnStart))
    (CallFunction|PatrolThroughAllPoints)))

(event Custom|GoToPosition
  (if (not (Variables|Default|GetPatrolingOnStart))
    (AI|AIMoveTo (AI|GetAIController self) "0, 0, 0" (.DestActor (Utilities|Struct|BreakPatrolDestination (Utilities|Array|Get(acopy) (Variables|Default|GetPatrolPoints)))) -1.0 "Default" "Default" true true
      (:OnMoveFinished
        (bind _alpha (Timeline|Timeline_0 PlayFromStart)
          (:Update
            (Transformation|SetActorRotation (Math|Rotator|Lerp(Rotator) (Transformation|GetActorRotation) (Transformation|GetActorRotation (.DestActor (Utilities|Struct|BreakPatrolDestination (Utilities|Array|Get(acopy) (Variables|Default|GetPatrolPoints))))) _alpha true))))))))

(event EventBeginPlay
  (CallFunction|BeginPatrolTest))

(event EventTick
  (params (DeltaSeconds :type Float%20%28single-precision%29))
  (CallFunction|RotateNametoPlayer))

(event EventOnLanded
  (params (Hit :type Hit%20Result%20Structure%20%28by%20ref%29))
  (if (> (Utilities|Array|Length (Variables|Default|GetPatrolPoints)) 0)
    (if (Variables|Default|GetPatrolingOnStart)
      (CallFunction|PatrolThroughAllPoints)
      (else
        (CallFunction|GotoPosition)))))

(fn ConstructionScript
  (bind _nmetypename (Variables|Default|GetNMETypeName))
  (Rendering|Material|SetVectorParameterValueonMaterials (Variables|Character|GetMesh) "BodyColor" (Math|Conversions|ToVector(LinearColor) (Variables|Default|GetBodyColor)))
  (Variables|/Script/Engine.CharacterMovementComponent|SetMaxWalkSpeed (Variables|Character|GetCharacterMovement) (Variables|Default|GetWalkSpeed))
  (Rendering|Components|TextRender|SetText (Variables|Default|GetNMEType) (Utilities|Text|ToText(String) _nmetypename))
  (Variables|/Game/Blueprints/Components/BP_InteractibleComponent.BP_InteractibleComponent_C|SetItemName (Variables|Default|GetBP_InteractibleComponent) _nmetypename))

(fn RotateNametoPlayer
  (bind _nmetype (Variables|Default|GetNMEType))
  (Transformation|SetWorldRotation _nmetype (Math|Rotator|FindLookatRotation (Transformation|GetWorldLocation _nmetype) (Transformation|GetActorLocation (Game|GetPlayerCameraManager 0))) false false))