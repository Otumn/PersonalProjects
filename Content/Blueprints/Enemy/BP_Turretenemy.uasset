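; Turret enemy Blueprint that fires projectiles at the player's camera and dies when attacked.
; ShootBlast aims the muzzle at the camera, spawns BP_EnemyProjectile and briefly raises a shooting flag.
; Timelines blend gun material color and point light between reloading and loaded looks, scaled to reload time, with cancellation fading back from the current light values.
; Being attacked disables capsule collision, cancels the effect and reports the kill to the game manager.
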(event OnAttacked(BP_AttackableComponent)
  (Utilities|FlowControl|Sequence
    (:then_0
      (Variables|StateBooleans|SetbIsDead? true)
      (Collision|SetCollisionEnabled (Variables|Collision|GetCapsuleComponent) "NoCollision"))
    (:then_1
      (CallFunction|CancelReloadEffect))
    (:then_2
      (Default|CallOnActorKilled (CallFunction|GetGameManager) self))))

(event Custom|ReloadEffect
  (bind _alpha (Timeline|ReloadEffectTimeline PlayFromStart)
    (:Update
      (Rendering|Material|SetVectorParameterValueonMaterials (Variables|Default|GetSK_FPGun) "BodyColor" (Math|Vector|Lerp(Vector) (Math|Conversions|ToVector(LinearColor) (Variables|Default|GetGunReloadingColor)) (Math|Conversions|ToVector(LinearColor) (Variables|Default|GetGunLoadedColor)) _alpha))
      (Rendering|Components|Light|SetLightColor (Variables|Default|GetPointLight) (Math|Color|Lerp(LinearColor) (Variables|Default|GetGunReloadingColor) (Variables|Default|GetGunLoadedColor) _alpha) true)
      (Rendering|Components|Light|SetIntensity (Variables|Default|GetPointLight) (Math|Float|Lerp (Variables|Default|GetLightReloadingIntensity) (Variables|Default|GetLightLoadedIntensity) _alpha)))))

(event Custom|CancelReloadEffect
  (bind _pointlight (Variables|Default|GetPointLight))
  (Utilities|FlowControl|Sequence
    (:then_0
      (bind _alpha (Timeline|ReloadEffectTimeline Stop)
        (:Update
          (Rendering|Material|SetVectorParameterValueonMaterials (Variables|Default|GetSK_FPGun) "BodyColor" (Math|Vector|Lerp(Vector) (Math|Conversions|ToVector(LinearColor) (Variables|Default|GetGunReloadingColor)) (Math|Conversions|ToVector(LinearColor) (Variables|Default|GetGunLoadedColor)) _alpha))
          (Rendering|Components|Light|SetLightColor (Variables|Default|GetPointLight) (Math|Color|Lerp(LinearColor) (Variables|Default|GetGunReloadingColor) (Variables|Default|GetGunLoadedColor) _alpha) true)
          (Rendering|Components|Light|SetIntensity (Variables|Default|GetPointLight) (Math|Float|Lerp (Variables|Default|GetLightReloadingIntensity) (Variables|Default|GetLightLoadedIntensity) _alpha)))))
    (:then_1
      (Variables|Default|SetCurrentColor (Rendering|Components|Light|GetLightColor _pointlight))
      (Variables|Default|SetCurrentIntensity (Variables|/Script/Engine.LightComponentBase|GetIntensity _pointlight)))
    (:then_2
      (bind _alpha_2 (Timeline|CancelReloadEffectTimeline PlayFromStart)
        (:Update
          (Rendering|Material|SetVectorParameterValueonMaterials (Variables|Default|GetSK_FPGun) "BodyColor" (Math|Vector|Lerp(Vector) (Math|Conversions|ToVector(LinearColor) (Variables|Default|GetCurrentColor)) (Math|Conversions|ToVector(LinearColor) (Variables|Default|GetGunReloadingColor)) _alpha_2))
          (Rendering|Components|Light|SetLightColor (Variables|Default|GetPointLight) (Math|Color|Lerp(LinearColor) (Variables|Default|GetCurrentColor) (Variables|Default|GetGunReloadingColor) _alpha_2) true)
          (Rendering|Components|Light|SetIntensity (Variables|Default|GetPointLight) (Math|Float|Lerp (Variables|Default|GetCurrentIntensity) (Variables|Default|GetLightReloadingIntensity) _alpha_2)))))))

(event Custom|ShootBlast
  (Variables|StateBooleans|SetbIsShooting? true)
  (Transformation|SetWorldRotation (Variables|Default|GetMuzzlePoint) (Math|Rotator|FindLookatRotation (Transformation|GetWorldLocation (Variables|Default|GetMuzzlePoint)) (Transformation|GetActorLocation (Game|GetPlayerCameraManager 0))) false false)
  (Game|SpawnActorfromClass "/Game/Blueprints/Enemy/BP_EnemyProjectile.BP_EnemyProjectile_C" (Transformation|GetWorldTransform (Variables|Default|GetMuzzlePoint)) "AlwaysSpawn" 0 0)
  (Utilities|FlowControl|Delay 0.233)
  (Variables|StateBooleans|SetbIsShooting? false))

(event EventBeginPlay
  (CallFunction|SetupEffects))

(fn ConstructionScript)

(fn SetupEffects
  (bind _pointlight (Variables|Default|GetPointLight))
  (bind _gunreloadingcolor (Variables|Default|GetGunReloadingColor))
  (Rendering|Material|SetVectorParameterValueonMaterials (Variables|Default|GetSK_FPGun) "BodyColor" (Math|Conversions|ToVector(LinearColor) _gunreloadingcolor))
  (Rendering|Components|Light|SetLightColor _pointlight _gunreloadingcolor true)
  (Rendering|Components|Light|SetIntensity _pointlight (Variables|Default|GetLightReloadingIntensity))
  (Components|Timeline|SetPlayRate (Variables|Default|GetCancelReloadEffectTimeline) (Variables|Default|GetCancelReloadEffectRate))
  (Components|Timeline|SetPlayRate (Variables|Default|GetReloadEffectTimeline) (/ 1.0 (Variables|Default|GetReloadTime))))