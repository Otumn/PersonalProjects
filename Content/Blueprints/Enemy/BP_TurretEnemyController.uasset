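; AI controller for the turret enemy that runs its behavior tree on possess and tracks whether it sees the player or is dead.
; Perception updates check the first sense against the player pawn, setting CanSeePlayer on the blackboard and HasTarget on the turret.
; Losing sight starts a timer that delays clearing the target, and regaining sight cancels it.
; It binds to the game manager's actor-killed event to set IsDead for its own pawn.
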(event OnPerceptionUpdated(AIPerception)
  (params (UpdatedActors :type Array%20of%20Actor%20Object%20References))
  (for _array_element UpdatedActors
    (bind _info (Class|AIPerceptionComponent|GetActorsPerception (Variables|Default|GetAIPerception) _array_element))
    (CallFunction|GoThroughSenses _info)))

(event Custom|SightLoss
  (CallFunction|UpdateCanSeePlayer false))

(event Custom|OnActorKilled
  (params (Actor :type Actor%20Object%20Reference))
  (if (== Actor (Pawn|GetControlledPawn))
    (CallFunction|UpdateIsDead true)))

(event EventPossess
  (params (PossessedPawn :type Pawn%20Object%20Reference))
  (AI|RunBehaviorTree "/Game/Blueprints/Enemy/BP_TurretEnemyBE.BP_TurretEnemyBE")
  (CallFunction|SetupEvents))

(fn ConstructionScript)

(fn GoThroughSenses
  (params (Infos :type Actor%20Perception%20Blueprint%20Info%20Structure))
  (bind (_target _lastsensedstimuli) (Utilities|Struct|BreakActorPerceptionBlueprintInfo Infos))
  (bind (_array_element _array_index) (Utilities|Array|ForEachLoopwithBreak _lastsensedstimuli)
    (:LoopBody
      (LocalVariables|SetTestedSense _array_element)
      (switch int _array_index
        (:0
          (if (== _target (Game|Player|GetPlayerPawn 0))
            (if (.bSuccessfullySensed (Utilities|Struct|BreakAIStimulus (LocalVariables|GetTestedSense)))
              (Utilities|Time|ClearandInvalidateTimerbyHandle (Variables|Default|GetLostSightTimer))
              (CallFunction|UpdateCanSeePlayer true)
              (else
                (bind _returnvalue (Utilities|Time|SetTimerbyEvent (EventDispatchers|CreateEvent :!event Custom|SightLoss) (Variables|Default|GetTimeBeforeLoseSight)))
                (Variables|Default|SetLostSightTimer _returnvalue)))))))))

(fn UpdateCanSeePlayer
  (params (bool :type Boolean))
  (AI|Components|Blackboard|SetValueasBool (AI|GetBlackboard 0) (Variables|BlackboardKeys|GetCanSeePlayer?) bool)
  (Variables|/Game/Blueprints/Enemy/BP_Turretenemy.BP_TurretEnemy_C|SetbHasTarget? (.AsBP%20Turret%20Enemy (Utilities|Casting|CastToBP_TurretEnemy (Pawn|GetControlledPawn))) bool))

(fn SetupEvents
  (EventDispatchers|BindEventtoOnActorKilled (CallFunction|GetGameManager) (EventDispatchers|CreateEvent :!event Custom|OnActorKilled)))

(fn UpdateIsDead
  (params (bool :type Boolean))
  (AI|Components|Blackboard|SetValueasBool (AI|GetBlackboard 0) (Variables|BlackboardKeys|GetIsDead?) bool))