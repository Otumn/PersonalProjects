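; Prison guard enemy that patrols waypoints or holds a post and detects the escapee player.
; Inside its detection sphere, a facing dot-product test plus body, feet and camera line traces start detection, stopping movement.
; Tick turns it toward the player and fills a camera-facing alert bar, notifying the game manager when full.
; Leaving the sphere drains the bar, then movement resumes; the camera trace overwrites SeesFeet, never setting SeesHead.
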(event OnComponentBeginOverlap(DetectionShere)
  (params (OverlappedComponent :type Primitive%20Component%20Object%20Reference) (OtherActor :type Actor%20Object%20Reference) (OtherComp :type Primitive%20Component%20Object%20Reference) (OtherBodyIndex :type Integer) (bFromSweep :type Boolean) (SweepResult :type Hit%20Result%20Structure%20%28by%20ref%29))
  (if (== OtherActor (Game|Player|GetPlayerPawn 0))
    (if (and (CallFunction|IsPlayerinFrontOf?) (CallFunction|BHasPlayerinSight?))
      (Variables|StateBooleans|SetbIsDetecting? true)
      (CallFunction|CancelMovement)
      (else
        (Variables|Detection|SetbHasToCheckForDetection? true)))))

(event OnComponentEndOverlap(DetectionShere)
  (params (OverlappedComponent :type Primitive%20Component%20Object%20Reference) (OtherActor :type Actor%20Object%20Reference) (OtherComp :type Primitive%20Component%20Object%20Reference) (OtherBodyIndex :type Integer))
  (if (== OtherActor (Game|Player|GetPlayerPawn 0))
    (if (Variables|StateBooleans|GetbIsDetecting?)
      (Variables|StateBooleans|SetbIsDetecting? false)
      (Variables|StateBooleans|SetbHasToLoseAlert? true)
      (Variables|Detection|SetbHasToCheckForDetection? false))))

(event Custom|PatrolThroughAllPoints
  (if (not (Variables|StateBooleans|GetbIsDetecting?))
    (bind _alpha (Timeline|TurnAroundTimeline PlayFromStart)
      (:Update
        (Transformation|SetActorRotation (Math|Rotator|Lerp(Rotator) (Transformation|GetActorRotation) (Transformation|GetActorRotation (.DestActor (Utilities|Struct|BreakPatrolDestination (Utilities|Array|Get(acopy) (Variables|Default|GetPatrolPoints) (Variables|Default|GetCurrentPatrolIndex))))) _alpha true)))
      (:Finished
        (Utilities|FlowControl|Delay (+ (.WaitTime (Utilities|Struct|BreakPatrolDestination (Utilities|Array|Get(acopy) (Variables|Default|GetPatrolPoints) (Variables|Default|GetCurrentPatrolIndex)))) (Math|Random|RandomFloatinRange -0.1 0.1)))
        (if (not (Variables|StateBooleans|GetbIsDetecting?))
          (Variables|Default|SetCurrentPatrolIndex (+ (Variables|Default|GetCurrentPatrolIndex) 1))
          (if (> (Variables|Default|GetCurrentPatrolIndex) (- (Utilities|Array|Length (Variables|Default|GetPatrolPoints)) 1))
            (Variables|Default|SetCurrentPatrolIndex 0))
          (CallFunction|GotoCurrentPatrolPoint))))))

(event Custom|BeginPatrolTest
  (if (Math|Boolean|ANDBoolean (> (Utilities|Array|Length (Variables|Default|GetPatrolPoints)) 0) (AI|Components|NavMovement|IsMovingonGround (Variables|Character|GetCharacterMovement)) (Variables|Default|GetPatrolingOnStart))
    (CallFunction|PatrolThroughAllPoints)))

(event Custom|GoToPosition
  (if (not (Variables|Default|GetPatrolingOnStart))
    (AI|AIMoveTo (AI|GetAIController self) "0, 0, 0" (.DestActor (Utilities|Struct|BreakPatrolDestination (Utilities|Array|Get(acopy) (Variables|Default|GetPatrolPoints)))) -1.0 "Default" "Default" true true
      (:OnMoveFinished
        (bind _alpha (Timeline|Timeline_0 PlayFromStart)
          (:Update
            (Transformation|SetActorRotation (Math|Rotator|Lerp(Rotator) (Transformation|GetActorRotation) (Transformation|GetActorRotation (.DestActor (Utilities|Struct|BreakPatrolDestination (Utilities|Array|Get(acopy) (Variables|Default|GetPatrolPoints))))) _alpha true))))))))

(event Custom|CancelMovement
  (AI|Navigation|StopMovement (AI|GetAIController self)))

(event Custom|GoToCurrentPatrolPoint
  (AI|AIMoveTo (AI|GetAIController self) "0, 0, 0" (.DestActor (Utilities|Struct|BreakPatrolDestination (Utilities|Array|Get(acopy) (Variables|Default|GetPatrolPoints) (Variables|Default|GetCurrentPatrolIndex)))) -1.0 "Default" "Default" true true
    (:OnMoveFinished
      (CallFunction|PatrolThroughAllPoints))))

(event EventBeginPlay
  (CallFunction|SetupBar)
  (CallFunction|BeginPatrolTest)
  (Math|Integer|IncrementInt (Variables|/Game/Blueprints/Player/Escapee/BP_EscapeePlayer.BP_EscapeePlayer_C|GetOriginalNbOfGuards (.AsBP%20Escapee%20Player (Utilities|Casting|CastToBP_EscapeePlayer (Game|Player|GetPlayerPawn 0))))))

(event EventTick
  (params (DeltaSeconds :type Float%20%28single-precision%29))
  (Variables|Default|SetDeltaTime DeltaSeconds)
  (CallFunction|RotateBartoPlayer)
  (CallFunction|DetectionManager))

(event EventOnLanded
  (params (Hit :type Hit%20Result%20Structure%20%28by%20ref%29))
  (if (> (Utilities|Array|Length (Variables|Default|GetPatrolPoints)) 0)
    (if (Variables|Default|GetPatrolingOnStart)
      (CallFunction|PatrolThroughAllPoints)
      (else
        (CallFunction|GotoPosition)))))

(fn ConstructionScript
  (Rendering|Material|SetVectorParameterValueonMaterials (Variables|Character|GetMesh) "BodyColor" (Math|Conversions|ToVector(LinearColor) (Variables|Default|GetBodyColor)))
  (Variables|/Script/Engine.CharacterMovementComponent|SetMaxWalkSpeed (Variables|Character|GetCharacterMovement) (Variables|Default|GetWalkSpeed)))

(fn RotateBartoPlayer
  (bind _alertbarwidget (Variables|Default|GetAlertBarWidget))
  (Transformation|SetWorldRotation _alertbarwidget (Math|Rotator|FindLookatRotation (Transformation|GetWorldLocation _alertbarwidget) (Transformation|GetActorLocation (Game|GetPlayerCameraManager 0))) false false))

(fn DetectionManager
  (bind _returnvalue (Game|Player|GetPlayerPawn 0))
  (bind _alertbar (Variables|Default|GetAlertBar))
  (bind _alertbar_2 (Variables|Default|GetAlertBar))
  (bind _detectionrate (Variables|Detection|GetDetectionRate))
  (bind _undetectionrate (Variables|Detection|GetUnDetectionRate))
  (bind _percent (Default|GetAlertProgress _alertbar))
  (bind _percent_2 (Default|GetAlertProgress _alertbar_2))
  (bind _asbp_escapee_player (Utilities|Casting|CastToBP_EscapeePlayer _returnvalue))
  (bind _multiplier (Default|GetDetectionMultiplier _asbp_escapee_player))
  (bind _returnvalue_2 (- _percent _undetectionrate))
  (bind _returnvalue_3 (Math|Float|Clamp(Float) _returnvalue_2))
  (bind _returnvalue_4 (* _detectionrate _multiplier))
  (bind _returnvalue_5 (+ _percent_2 _returnvalue_4))
  (bind _returnvalue_6 (Math|Float|Clamp(Float) _returnvalue_5))
  (if (Variables|StateBooleans|GetbIsDetecting?)
    (Utilities|FlowControl|Sequence
      (:then_0
        (Default|SetAlertProgress _alertbar_2 _returnvalue_6)
        (if (>= _returnvalue_6 1.0)
          (Default|CallOnPlayerDetected (CallFunction|GetGameManager))))
      (:then_1
        (Transformation|SetActorRotation (Math|Interpolation|RInterpTo (Transformation|GetActorRotation) (Math|Rotator|FindLookatRotation (Transformation|GetActorLocation) (Transformation|GetActorLocation (Game|Player|GetPlayerPawn 0))) (Variables|Default|GetDeltaTime) (Variables|Detection|GetTurnAroundSpeed)))))
    (else
      (Utilities|FlowControl|Sequence
        (:then_0
          (if (Variables|StateBooleans|GetbHasToLoseAlert?)
            (Default|SetAlertProgress _alertbar _returnvalue_3)
            (if (<= _returnvalue_3 0.0)
              (CallFunction|GotoCurrentPatrolPoint)
              (Variables|StateBooleans|SetbHasToLoseAlert? false))))
        (:then_1
          (if (Variables|Detection|GetbHasToCheckForDetection?)
            (if (and (CallFunction|IsPlayerinFrontOf?) (CallFunction|BHasPlayerinSight?))
              (Variables|StateBooleans|SetbIsDetecting? true)
              (CallFunction|CancelMovement))))))))

(fn SetupBar
  (Variables|Default|SetAlertBar (.AsBP%20Prison%20Guard%20Widget (Utilities|Casting|CastToBP_PrisonGuardWidget (UserInterface|GetUserWidgetObject (Variables|Default|GetAlertBarWidget))))))

(fn IsPlayerinFrontOf?
  (return (> (Math|Vector|DotProduct (Math|Vector|Normalize (- (Transformation|GetActorLocation (Game|Player|GetPlayerPawn 0)) (Transformation|GetActorLocation))) (Math|Vector|GetForwardVector (Variables|Collision|GetCapsuleComponent))) (Variables|Detection|GetDetectionThreshhold))))

(fn BHasPlayerinSight?
  (bind _returnvalue (Transformation|GetActorLocation))
  (bind _returnvalue_2 (Transformation|GetActorLocation))
  (bind _returnvalue_3 (Transformation|GetActorLocation))
  (Utilities|FlowControl|Sequence
    (:then_0
      (bind (_outhit _returnvalue_4) (Collision|LineTraceByChannel _returnvalue (+ (* (Math|Vector|Normalize (- (Transformation|GetActorLocation (Game|Player|GetPlayerPawn 0)) (Transformation|GetActorLocation))) (Variables|/Script/Engine.SphereComponent|GetSphereRadius (Variables|Default|GetDetectionShere))) _returnvalue) "TraceTypeQuery1" false 0 "ForOneFrame"))
      (if _returnvalue_4
        (LocalVariables|SetbSeesBody? (== (.HitActor (Collision|BreakHitResult _outhit)) (Game|Player|GetPlayerPawn 0)))))
    (:then_1
      (bind (_outhit_2 _returnvalue_5) (Collision|LineTraceByChannel _returnvalue_2 (+ _returnvalue_2 (* (Math|Vector|Normalize (- (Transformation|GetWorldLocation (Variables|/Game/Blueprints/Player/Escapee/BP_EscapeePlayer.BP_EscapeePlayer_C|GetFeetMarker (.AsBP%20Escapee%20Player (Utilities|Casting|CastToBP_EscapeePlayer (Game|Player|GetPlayerPawn 0))))) (Transformation|GetActorLocation))) (Variables|/Script/Engine.SphereComponent|GetSphereRadius (Variables|Default|GetDetectionShere)))) "TraceTypeQuery1" false 0 "ForOneFrame" true "(R=0.000000,G=0.097294,B=1.000000,A=1.000000)"))
      (if _returnvalue_5
        (LocalVariables|SetbSeesFeet? (== (.HitActor (Collision|BreakHitResult _outhit_2)) (Game|Player|GetPlayerPawn 0)))))
    (:then_2
      (bind (_outhit_3 _returnvalue_6) (Collision|LineTraceByChannel _returnvalue_3 (+ _returnvalue_3 (* (Math|Vector|Normalize (- (Transformation|GetActorLocation (Game|GetPlayerCameraManager 0)) (Transformation|GetActorLocation))) (Variables|/Script/Engine.SphereComponent|GetSphereRadius (Variables|Default|GetDetectionShere)))) "TraceTypeQuery1" false 0 "ForOneFrame" true "(R=0.006027,G=1.000000,B=0.000000,A=1.000000)"))
      (if _returnvalue_6
        (LocalVariables|SetbSeesFeet? (== (.HitActor (Collision|BreakHitResult _outhit_3)) (Game|Player|GetPlayerPawn 0)))))
    (:then_3
      (return (Math|Boolean|ORBoolean (LocalVariables|GetbSeesBody?) (LocalVariables|GetbSeesFeet?) (LocalVariables|GetbSeesHead?))))))