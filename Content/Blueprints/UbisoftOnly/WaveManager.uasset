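; Wave manager that runs three enemy waves between objectives 1 and 2, announcing each through the game manager.
; Pre-placed enemies are pooled by toggling visibility, collision, tick and gravity, then sent to position when shown.
; Objective 1 starts the first wave; the N key advances manually, while B toggles a separate Wave 0 group.
; Wave 3 hides the hangar door and drives a jeep along a spline by timeline before revealing its enemies.
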(event Custom|StartWave3
  (bind _hangardoor (Variables|Default|GetHangarDoor))
  (Rendering|SetActorHiddenInGame _hangardoor true)
  (Collision|SetActorEnableCollision _hangardoor false)
  (Actor|Tick|SetActorTickEnabled _hangardoor)
  (bind (_direction _locationalpha _rotationalpha) (Timeline|JeepArrival PlayFromStart)
    (:Update
      (Transformation|SetActorLocationAndRotation (Variables|Default|GetJeep) (Spline|GetLocationatTime (Variables|Default|GetSpline) _locationalpha "World" true) (Math|Rotator|Lerp(Rotator) (Math|Rotator|MakeRotator 0.0 0.0 (Variables|Default|GetJeepStartAngle)) (Math|Rotator|MakeRotator 0.0 0.0 (Variables|Default|GetJeepTargetAngle)) _rotationalpha true) false true))
    (:Finished
      (CallFunction|ClassicWaveStart (Variables|Default|GetWave3Enemies)))))

(event Custom|StartWave1
  (CallFunction|ClassicWaveStart (Variables|Default|GetWave1Enemies)))

(event Custom|HideWave0
  (CallFunction|ClassicWaveHide (Variables|Default|GetWave0Enemies)))

(event Custom|OnNewObjective
  (params (Index :type Integer))
  (if (== Index 1)
    (Variables|Default|SetbAreWavesActive? true)
    (Utilities|FlowControl|Sequence
      (:then_0
        (CallFunction|StartNextWave))
      (:then_1
        (Math|Integer|IncrementInt (Variables|Default|GetCurrentWaveIndex))))))

(event Custom|HideWave3
  (CallFunction|ClassicWaveHide (Variables|Default|GetWave3Enemies))
  (bind (_direction _locationalpha _rotationalpha) (Timeline|JeepArrival Stop)
    (:Update
      (Transformation|SetActorLocationAndRotation (Variables|Default|GetJeep) (Spline|GetLocationatTime (Variables|Default|GetSpline) _locationalpha "World" true) (Math|Rotator|Lerp(Rotator) (Math|Rotator|MakeRotator 0.0 0.0 (Variables|Default|GetJeepStartAngle)) (Math|Rotator|MakeRotator 0.0 0.0 (Variables|Default|GetJeepTargetAngle)) _rotationalpha true) false true))
    (:Finished
      (CallFunction|ClassicWaveStart (Variables|Default|GetWave3Enemies)))))

(event Custom|StartWave2
  (CallFunction|ClassicWaveStart (Variables|Default|GetWave2Enemies)))

(event Custom|HideWave1
  (CallFunction|ClassicWaveHide (Variables|Default|GetWave1Enemies)))

(event Custom|HideAllActors
  (CallFunction|ClassicWaveHide (Variables|Default|GetWave1Enemies))
  (CallFunction|ClassicWaveHide (Variables|Default|GetWave2Enemies))
  (CallFunction|ClassicWaveHide (Variables|Default|GetWave3Enemies)))

(event Custom|HideWave2
  (CallFunction|ClassicWaveHide (Variables|Default|GetWave2Enemies)))

(event Custom|StartNextWave
  (switch int (Variables|Default|GetCurrentWaveIndex)
    (:0
      (CallFunction|StartWave1)
      (Default|CallOnGameMessage (CallFunction|GetGameManager) "Wave 1 "))
    (:1
      (CallFunction|HideWave1)
      (CallFunction|StartWave2)
      (Default|CallOnGameMessage (CallFunction|GetGameManager) "Wave 2 "))
    (:2
      (CallFunction|HideWave2)
      (CallFunction|StartWave3)
      (Default|CallOnGameMessage (CallFunction|GetGameManager) "Wave 3 "))
    (:3
      (CallFunction|HideWave3)
      (Default|CallOnGameMessage (CallFunction|GetGameManager))
      (Default|CallOnObjectiveSet (CallFunction|GetGameManager) 2))))

(event EventBeginPlay
  (CallFunction|HideAllActors)
  (Input|EnableInput (Game|GetPlayerController 0))
  (EventDispatchers|BindEventtoOnObjectiveSet (CallFunction|GetGameManager) (EventDispatchers|CreateEvent :!event Custom|OnNewObjective))
  (Utilities|FlowControl|Delay 0.2)
  (Default|CallOnObjectiveSet (CallFunction|GetGameManager) 0))

(event Input|KeyboardEvents|N
  (params (Key :type Key%20Structure :default "None"))
  (:Pressed
    (if (Variables|Default|GetbAreWavesActive?)
      (Utilities|FlowControl|Sequence
        (:then_0
          (CallFunction|StartNextWave))
        (:then_1
          (Math|Integer|IncrementInt (Variables|Default|GetCurrentWaveIndex)))))))

(event Input|KeyboardEvents|B
  (params (Key :type Key%20Structure :default "None"))
  (bind _wave0enemies (Variables|Default|GetWave0Enemies))
  (:Pressed
    (Utilities|FlowControl|FlipFlop
      (:A
        (CallFunction|ClassicWaveHide _wave0enemies))
      (:B
        (CallFunction|ClassicWaveStart _wave0enemies)))))

(fn ConstructionScript)

(fn ClassicWaveHide
  (params (Array :type Array%20of%20BP%20Patrol%20Enemy%20Object%20References))
  (for _array_element Array
    (Utilities|IsValid _array_element
      (:Is%20Valid
        (Rendering|SetActorHiddenInGame _array_element true)
        (Collision|SetActorEnableCollision _array_element false)
        (Actor|Tick|SetActorTickEnabled _array_element)
        (Variables|/Script/Engine.CharacterMovementComponent|SetGravityScale (Variables|/Script/Engine.Character|GetCharacterMovement _array_element) 0.0)))))

(fn ClassicWaveStart
  (params (Array :type Array%20of%20BP%20Patrol%20Enemy%20Object%20References))
  (for _array_element Array
    (Utilities|IsValid _array_element
      (:Is%20Valid
        (Rendering|SetActorHiddenInGame _array_element false)
        (Collision|SetActorEnableCollision _array_element true)
        (Actor|Tick|SetActorTickEnabled _array_element true)
        (Variables|/Script/Engine.CharacterMovementComponent|SetGravityScale (Variables|/Script/Engine.Character|GetCharacterMovement _array_element) 1.0)
        (Default|GotoPosition _array_element)))))