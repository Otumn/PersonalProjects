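; BP_IceCone is an ice cone that grows each time its iceable component reports being iced.
; Each OnIced event from BP_IceableComponent adds a uniform increment to the Scene component's relative scale, computed from AddedScale times Scaler.
; Scaler then drops by a small fixed step down to a clamped minimum, so growth slows with repeated icing but never stops.
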(event OnIced(BP_IceableComponent)
  (bind _scene (Variables|Default|GetScene))
  (Transformation|SetRelativeScale3D _scene (+ (Variables|/Script/Engine.SceneComponent|GetRelativeScale3D _scene) (Math|Vector|MakeVector (* (Variables|Default|GetAddedScale) (Variables|Default|GetScaler)) (* (Variables|Default|GetAddedScale) (Variables|Default|GetScaler)) (* (Variables|Default|GetAddedScale) (Variables|Default|GetScaler)))))
  (Variables|Default|SetScaler (Math|Float|Clamp(Float) (- (Variables|Default|GetScaler) 0.002) 0.01)))

(fn ConstructionScript)