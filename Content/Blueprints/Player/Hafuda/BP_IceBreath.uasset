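; BP_IceBreath is the player's ice breath actor, which freezes what it touches and expires beyond a maximum range.
; Each tick a sphere trace finds hits, calling OnIced on actors with BP_IceableComponent and destroying the breath.
; Hits without a valid actor spawn an ice block aligned to the impact normal and breath direction.
; Logic for extending a grown BP_IceBlock is present but unwired.
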(event EventTick
  (params (DeltaSeconds :type Float%20%28single-precision%29))
  (bind _returnvalue (Transformation|GetActorForwardVector))
  (bind _returnvalue_2 (Transformation|GetActorLocation))
  (bind _returnvalue_3 (Transformation|GetActorForwardVector))
  (bind _sphere (Variables|Default|GetSphere))
  (bind (_x _y _z) (Math|Vector|BreakVector _returnvalue_3))
  (bind _sphereradius (Variables|/Script/Engine.SphereComponent|GetSphereRadius _sphere))
  (Utilities|FlowControl|Sequence
    (:then_0
      ;[0 1 0] Sphere cast to test collisions
      (bind (_outhit _returnvalue_4) (Collision|SphereTraceByChannel (+ _returnvalue_2 (* _returnvalue _sphereradius)) (+ _returnvalue_2 (* _returnvalue (* _sphereradius -1.0))) _sphereradius "TraceTypeQuery1" false 0 "None"))
      (if _returnvalue_4
        (Utilities|IsValid (.HitActor (Collision|BreakHitResult _outhit))
          (:Is%20Valid
            ;[0 1 0] If the hit actor has an iceabl comp, we call on iced
            (if (.HasComponent (CallFunction|DoesActorHasComponent? (.HitActor (Collision|BreakHitResult _outhit)) "/Game/Blueprints/Components/BP_IceableComponent.BP_IceableComponent_C"))
              (Default|CallOnIced (.AsBP%20Iceable%20Component (Utilities|Casting|CastToBP_IceableComponent (.ReturnedComponent (CallFunction|DoesActorHasComponent? (.HitActor (Collision|BreakHitResult _outhit)) "/Game/Blueprints/Components/BP_IceableComponent.BP_IceableComponent_C")))) (.HitComponent (Collision|BreakHitResult _outhit)))
              (Actor|DestroyActor)))
          (:Is%20Not%20Valid
            ;[0 1 0] If the hit actor is none of that, spawn an ice block
            (Game|SpawnActorfromClass "/Game/Blueprints/Player/Hafuda/BP_IceBlock.BP_IceBlock_C" (Math|Transform|MakeTransform (.ImpactPoint (Collision|BreakHitResult _outhit)) (Math|Rotator|MakeRotationfromAxes (Math|Vector|Normalize (Math|Vector|MakeVector (* _x (Math|Float|Absolute(Float) (- (Math|Float|Absolute(Float) (.X (Math|Vector|BreakVector (.ImpactNormal (Collision|BreakHitResult _outhit))))) 1.0))) (* _y (Math|Float|Absolute(Float) (- (Math|Float|Absolute(Float) (.Y (Math|Vector|BreakVector (.ImpactNormal (Collision|BreakHitResult _outhit))))) 1.0))) (* _z (Math|Float|Absolute(Float) (- (Math|Float|Absolute(Float) (.Z (Math|Vector|BreakVector (.ImpactNormal (Collision|BreakHitResult _outhit))))) 1.0))))) (* (Math|Vector|CrossProduct (Math|Vector|Normalize (Math|Vector|MakeVector (* _x (Math|Float|Absolute(Float) (- (Math|Float|Absolute(Float) (.X (Math|Vector|BreakVector (.ImpactNormal (Collision|BreakHitResult _outhit))))) 1.0))) (* _y (Math|Float|Absolute(Float) (- (Math|Float|Absolute(Float) (.Y (Math|Vector|BreakVector (.ImpactNormal (Collision|BreakHitResult _outhit))))) 1.0))) (* _z (Math|Float|Absolute(Float) (- (Math|Float|Absolute(Float) (.Z (Math|Vector|BreakVector (.ImpactNormal (Collision|BreakHitResult _outhit))))) 1.0))))) (.ImpactNormal (Collision|BreakHitResult _outhit))) -1.0) (.ImpactNormal (Collision|BreakHitResult _outhit)))) "AlwaysSpawn" 0 "0.000000,0.000000,0.000000" 0)
            (Actor|DestroyActor)))))
    (:then_1
      ;[0 1 0] Distance check
      (if (> (Math|Vector|Distance(Vector) (Variables|Default|GetStartPos) (Transformation|GetActorLocation)) (Variables|Default|GetMaxRange))
        (Actor|DestroyActor)))))

(fn ConstructionScript)