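; BP_FireBreath is a player fire breath actor that ignites fireable objects it touches and has a limited range.
; It spawns at BeginAmplitude scale and eases toward full scale every tick.
; Each tick it sphere-traces through its own sphere on the Visibility channel, calling CallOnFired on any hit actor's BP_FireableComponent.
; It destroys itself once farther than MaxRange from StartPos.
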(event EventTick
  (params (DeltaSeconds :type Float%20%28single-precision%29))
  (bind _returnvalue (Transformation|GetActorForwardVector))
  (bind _returnvalue_2 (Transformation|GetActorLocation))
  (bind _sphere (Variables|Default|GetSphere))
  (bind _sphereradius (Variables|/Script/Engine.SphereComponent|GetSphereRadius _sphere))
  (Utilities|FlowControl|Sequence
    (:then_0
      (Transformation|SetActorScale3D (Math|Interpolation|VInterpTo (Transformation|GetActorScale3D) "1.000000,1.000000,1.000000" DeltaSeconds 2.0)))
    (:then_1
      (bind (_outhit _returnvalue_3) (Collision|SphereTraceByChannel (+ _returnvalue_2 (* _returnvalue _sphereradius)) (+ _returnvalue_2 (* _returnvalue (* _sphereradius -1.0))) _sphereradius "TraceTypeQuery1" false 0 "None"))
      (if _returnvalue_3
        (Utilities|IsValid (.HitActor (Collision|BreakHitResult _outhit))
          (:Is%20Valid
            (if (.HasComponent (CallFunction|DoesActorHasComponent? (.HitActor (Collision|BreakHitResult _outhit)) "/Game/Blueprints/Components/BP_FireableComponent.BP_FireableComponent_C"))
              (Default|CallOnFired (.AsBP%20Fireable%20Component (Utilities|Casting|CastToBP_FireableComponent (.ReturnedComponent (CallFunction|DoesActorHasComponent? (.HitActor (Collision|BreakHitResult _outhit)) "/Game/Blueprints/Components/BP_FireableComponent.BP_FireableComponent_C"))))))))))
    (:then_2
      (if (> (Math|Vector|Distance(Vector) (Variables|Default|GetStartPos) (Transformation|GetActorLocation)) (Variables|Default|GetMaxRange))
        (Actor|DestroyActor)))))

(event EventBeginPlay
  (bind _beginamplitude (Variables|Default|GetBeginAmplitude))
  (Transformation|SetActorScale3D (Math|Vector|MakeVector _beginamplitude _beginamplitude _beginamplitude)))

(fn ConstructionScript)