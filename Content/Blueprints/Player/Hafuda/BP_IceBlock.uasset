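; BP_IceBlock is an ice block actor that grows in on spawn and reacts to fire and ice hits.
; A timeline, paced by GrowthRate, scales the Block from zero to full size and records progress in GrowthValue.
; Firing destroys the actor through its fireable component.
; Icing any component other than Block spawns another ice block offset along that component's negative up vector, then removes that component, letting blocks chain.
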(event OnFired(BP_FireableComponent)
  (Actor|DestroyActor))

(event OnIced(BP_IceableComponent)
  (params (HitComponent :type Actor%20Component%20Object%20Reference))
  (bind _asscene_component (Utilities|Casting|CastToSceneComponent HitComponent))
  (if (not (== HitComponent (Variables|Default|GetBlock)))
    (Development|PrintString "new block!")
    (Game|SpawnActorfromClass "BP_IceBlock_C" (Math|Transform|MakeTransform (+ (* (Math|Vector|GetUpVector _asscene_component) -5e+01) (Transformation|GetWorldLocation _asscene_component)) (Transformation|GetWorldRotation _asscene_component)) "Undefined" 0 0)
    (Components|DestroyComponent HitComponent)))

(event EventBeginPlay
  (Components|Timeline|SetPlayRate (Variables|Default|GetGrowthTimeline) (Variables|Default|GetgrowthRate))
  (bind _alpha (Timeline|GrowthTimeline PlayFromStart)
    (:Update
      (Transformation|SetRelativeScale3D (Variables|Default|GetBlock) (Math|Vector|Lerp(Vector) "0, 0, 0" "1.000000,1.000000,1.000000" _alpha))
      (Variables|Default|SetgrowthValue _alpha))))

(fn ConstructionScript)