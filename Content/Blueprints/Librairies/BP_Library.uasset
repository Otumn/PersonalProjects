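; BP_Library is a Blueprint function library of small shared gameplay helpers.
; It returns the game instance cast to BP_GameManager, checks whether an actor has a component of a given class and returns it, and snaps one actor's rotation to look at another.
; GetSlopeDirection rotates the flattened slope normal by GetSlopeDegreeAngles results, with pitch fed to roll and roll to pitch, yielding a normalized direction.
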(fn GetGameManager
  (return (.AsBP%20Game%20Manager (Utilities|Casting|CastToBP_GameManager (Game|GetGameInstance)))))

(fn GetSlopeDirection
  (params (ReferenceRightVector :type Vector) (SlopeNormal :type Vector) (ReferenceUpVector :type Vector))
  (bind (_x _y) (Math|Vector|BreakVector SlopeNormal))
  (bind (_outslopepitchdegreeangle _outsloperolldegreeangle) (Class|KismetMathLibrary|GetSlopeDegreeAngles ReferenceRightVector SlopeNormal ReferenceUpVector))
  (return (Math|Vector|Normalize (Math|Vector|RotateVector (Math|Vector|Normalize (Math|Vector|MakeVector _x _y 0.0)) (Math|Rotator|MakeRotator _outslopepitchdegreeangle _outsloperolldegreeangle 0.0)))))

(fn DoesActorHasComponent?
  (params (TargetActor :type Actor%20Object%20Reference) (TargetComponent :type Actor%20Component%20Class%20Reference))
  (bind _returnvalue (Actor|GetComponentbyClass TargetActor TargetComponent))
  (Utilities|IsValid _returnvalue
    (:Is%20Valid
      (return true _returnvalue))
    (:Is%20Not%20Valid
      (return false 0))))

(fn ActorFaceActor
  (params (ActorToRotate :type Actor%20Object%20Reference) (Target :type Actor%20Object%20Reference))
  (Transformation|SetActorRotation ActorToRotate (Math|Rotator|FindLookatRotation (Transformation|GetActorLocation ActorToRotate) (Transformation|GetActorLocation Target))))