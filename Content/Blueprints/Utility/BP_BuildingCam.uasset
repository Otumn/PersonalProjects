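; BP_BuildingCam is a utility actor, apparently a building camera, carrying spiral and tiers overlay planes that look like composition guides.
; All logic runs in the Construction Script, which pushes each plane's color and opacity to its materials.
; It also yaws the spiral plane, scales it to a 16:9 ratio and mirrors it through a negative Y scale when Inverted is set.
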(event EventBeginPlay)

(event Collision|EventActorBeginOverlap
  (params (OtherActor :type Actor%20Object%20Reference)))

(event EventTick
  (params (DeltaSeconds :type Float%20%28single-precision%29)))

(fn ConstructionScript
  (bind _tiersplane (Variables|Default|GetTiersPlane))
  (Utilities|FlowControl|Sequence
    (:then_0
      (Rendering|Material|SetVectorParameterValueonMaterials (Variables|Default|GetSpiralPlane) "Color" (Math|Conversions|ToVector(LinearColor) (Variables|Default|GetSpiralColor)))
      (Rendering|Material|SetScalarParameterValueonMaterials (Variables|Default|GetSpiralPlane) "Opacity" (Variables|Default|GetSpiralOpacity))
      (Rendering|Material|SetVectorParameterValueonMaterials _tiersplane "Color" (Math|Conversions|ToVector(LinearColor) (Variables|Default|GetTiersColor)))
      (Rendering|Material|SetScalarParameterValueonMaterials _tiersplane "Opacity" (Variables|Default|GetTiersOpacity)))
    (:then_1
      (Transformation|SetRelativeRotation (Variables|Default|GetSpiralPlane) (Math|Rotator|MakeRotator 0.0 0.0 (Variables|Default|GetSpiralRotation)) false false))
    (:then_2
      (Transformation|SetRelativeScale3D (Variables|Default|GetSpiralPlane) (Math|Vector|MakeVector 1.77777 (Math|Float|SelectFloat -1.0 1.0 (Variables|Default|GetbInverted?)) 1.0)))))