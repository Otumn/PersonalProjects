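; BP_DevCamera is a developer camera tool with toggles for a black-and-white look and a depth-of-field blur.
; ToggleBaW flips the stored saturation between full color and grayscale, while ToggleBlur flips the stored focal distance between zero and a fixed value.
; Both events feed one shared step that rebuilds the camera's post-process settings from both values, so each effect persists when the other toggles.
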(event Custom|ToggleBlur
  (if (== (Variables|Default|GetCurrentBlur) 0.0)
    (Variables|Default|SetCurrentBlur 6.5)
    (else
      (Variables|Default|SetCurrentBlur 0.0)))
  (Variables|/Script/Engine.CameraComponent|SetPostProcessSettings (Variables|Default|GetCamera) (Utilities|Struct|MakePostProcessSettings (Variables|Default|GetCurrentSaturation) (Variables|Default|GetCurrentBlur))))

(event Custom|ToggleBaW
  (if (== (.X (Math|Vector4|BreakVector4 (Variables|Default|GetCurrentSaturation))) 0.0)
    (Variables|Default|SetCurrentSaturation (Math|Vector4|MakeVector4 1.0 1.0 1.0 1.0))
    (else
      (Variables|Default|SetCurrentSaturation (Math|Vector4|MakeVector4 0.0 0.0 0.0 1.0))))
  (Variables|/Script/Engine.CameraComponent|SetPostProcessSettings (Variables|Default|GetCamera) (Utilities|Struct|MakePostProcessSettings (Variables|Default|GetCurrentSaturation) (Variables|Default|GetCurrentBlur))))

(fn ConstructionScript)